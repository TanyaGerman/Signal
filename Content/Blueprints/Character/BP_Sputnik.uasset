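; BP_Sputnik is a player character that starts running forward automatically after the first forward input and can jump.
; BeginPlay adds the IMC_Move Enhanced Input mapping context through MyController.
; The first IA_Forward trigger sets IsAutoMove, nudges along actor forward and starts a looping timer calling AutoMove, which feeds movement input along world forward.
; Nothing here stops the auto-move; IA_Jump sets a jumping flag and calls Jump.
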(event Input|EnhancedActionEvents|EnhancedInputActionIA_Forward
  (params (ActionValue :type Float%20%28double-precision%29) (ElapsedSeconds :type Float%20%28double-precision%29) (TriggeredSeconds :type Float%20%28double-precision%29) (InputAction :type Input%20Action%20Object%20Reference :default "/Game/Blueprints/Character/IA_Forward.IA_Forward"))
  (:Triggered
    (if (not (Variables|Default|GetIsAutoMove))
      (Variables|Default|SetIsAutoMove true)
      (Utilities|Time|SetTimerbyFunctionName 0 "AutoMove" 0.02 true)
      (Pawn|Input|AddMovementInput (Transformation|GetActorForwardVector) 1.0 false))))

(event Input|EnhancedActionEvents|EnhancedInputActionIA_Jump
  (params (ActionValue :type Boolean) (ElapsedSeconds :type Float%20%28double-precision%29) (TriggeredSeconds :type Float%20%28double-precision%29) (InputAction :type Input%20Action%20Object%20Reference :default "/Game/Blueprints/Character/IA_Jump.IA_Jump"))
  (Variables|Default|SetblsJumping true)
  (Character|Jump))

(event EventBeginPlay
  (bind _ascontroller (Utilities|Casting|CastToMyController (Pawn|GetController)))
  (Input|AddMappingContext (PlayerController|LocalPlayerSubsystems|GetEnhancedInputLocalPlayerSubsystem _ascontroller) "/Game/Blueprints/Character/IMC_Move.IMC_Move" 0 "(bIgnoreAllPressedKeysUntilRelease=True,bForceImmediately=False,bNotifyUserSettings=False)"))

(fn ConstructionScript)

(fn AutoMove
  (Pawn|Input|AddMovementInput (Class|KismetMathLibrary|VectorForward) 1.0 false))