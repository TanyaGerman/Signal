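; Player camera manager that drives a fixed-rotation, fixed-FOV side-view camera following the view target with smoothed movement.
; Each update, a radial fan of line traces in the XZ plane finds the nearest static or dynamic world object around the target.
; That distance feeds a curve giving the camera's arm length along Y, so zoom adapts to surrounding space.
; Arm length and camera location are both interpolated before overriding the camera view.
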(event EventBeginPlay)

(event Collision|EventActorBeginOverlap
  (params (OtherActor :type Actor%20Object%20Reference)))

(event EventTick
  (params (DeltaSeconds :type Float%20%28single-precision%29)))

(fn ConstructionScript)

(fn BlueprintUpdateCamera
  (params (CameraTarget :type Actor%20Object%20Reference))
  (Utilities|FlowControl|Sequence
    (:then_0
      (bind _mindistance (CallFunction|GetClosestCollisionPoint (Transformation|GetActorLocation CameraTarget)))
      (LocalVariables|Set-TergetArmLength (Math|Curves|GetFloatValue (Variables|Default|GetCameraDistanceCurve) _mindistance))
      (Variables|Default|SetCurrentArmLength (Math|Interpolation|FInterpTo (Variables|Default|GetCurrentArmLength) (LocalVariables|Get-TergetArmLength) (Utilities|Time|GetWorldDeltaSeconds) 4.0)))
    (:then_1
      (Variables|Default|SetCurrent%20CamLoc (Math|Interpolation|VInterpTo (Variables|Default|GetCurrent%20CamLoc) (+ (Transformation|GetActorLocation CameraTarget) "1000.000000,1200.000000,100.000000" (Math|Vector|MakeVector 0.0 (Variables|Default|GetCurrentArmLength) 0.0)) (Utilities|Time|GetWorldDeltaSeconds) 5.0)))
    (:then_2
      (return (Variables|Default|GetCurrent%20CamLoc) "0.000000,-90.000000,0.000000" 65.0 true))))

(fn GetClosestCollisionPoint
  (params (PlayerLocation :type Vector))
  (for _index (range 0 80)
    (bind (_outhit _returnvalue) (Collision|LineTraceForObjects PlayerLocation (+ PlayerLocation (* (Math|Vector|RotateVectorAroundAxis "1.000000,0.000000,0.000000" (Math|Conversions|ToFloat(Integer) (* _index 5)) "0.000000,1.000000,0.000000") (Math|Float|MakeLiteralFloat 3e+03))) (Utilities|Array|MakeArray "ObjectTypeQuery1" "ObjectTypeQuery2") false (Utilities|Array|MakeArray (Game|Player|GetPlayerPawn 0)) "None" true "(R=0.979978,G=0.135432,B=1.000000,A=1.000000)"))
    (if _returnvalue
      (if (< (.Distance (Collision|BreakHitResult _outhit)) (LocalVariables|Get-MinDistance))
        (LocalVariables|Set-MinDistance (.Distance (Collision|BreakHitResult _outhit))))))
  (return (LocalVariables|Get-MinDistance)))