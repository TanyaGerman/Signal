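; BP_Parralax is a background actor, named for parallax, that follows the player camera on X and Z while keeping its starting Y.
; BeginPlay caches the camera, actor and four layer component locations (03 to 06), and Tick moves the whole actor by the camera's displacement since then.
; The per-layer offset code with Layer03 to Layer05 multipliers is disconnected and fed zero vectors, so no layer moves independently.
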(event EventBeginPlay
  (Variables|Default|SetCameraLocation (Camera|GetCameraLocation (Game|GetPlayerCameraManager 0)))
  (Variables|Default|SetBackgroundLocation (Transformation|GetActorLocation))
  (Variables|Default|SetLayer06Loc (Transformation|GetWorldLocation (Variables|Default|Get06)))
  (Variables|Default|SetLayer05Loc (Transformation|GetWorldLocation (Variables|Default|Get05)))
  (Variables|Default|SetLayer04Loc (Transformation|GetWorldLocation (Variables|Default|Get04)))
  (Variables|Default|SetLayer03Loc (Transformation|GetWorldLocation (Variables|Default|Get03))))

(event EventTick
  (params (DeltaSeconds :type Float%20%28single-precision%29))
  (bind _output_get (Variables|Default|SetDeltaCam (- (Camera|GetCameraLocation (Game|GetPlayerCameraManager 0)) (Variables|Default|GetCameraLocation))))
  (Transformation|SetActorLocation (Math|Vector|MakeVector (.X (Math|Vector|BreakVector (+ _output_get (Variables|Default|GetBackgroundLocation)))) (.Y (Math|Vector|BreakVector (Variables|Default|GetBackgroundLocation))) (.Z (Math|Vector|BreakVector (+ _output_get (Variables|Default|GetBackgroundLocation))))) false false))

(fn ConstructionScript)