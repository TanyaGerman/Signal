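; Pawn with hand-written velocity movement that falls under gravity, slides along surfaces in the XZ plane and gets an upward impulse from Space.
; Each tick adds gravity to SputnikVelocity, pushes the pawn out of nearby geometry via a sphere trace, then applies a swept local offset.
; A velocity-direction trace redirects motion along the hit tangent, with speed scaled by a curve of their dot product.
; Debug drawing and prints remain, alongside disconnected normal-velocity experiments.
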(event EventTick
  (params (DeltaSeconds :type Float%20%28single-precision%29))
  (bind _returnvalue (Transformation|GetActorLocation))
  (bind _returnvalue_2 (Math|Float|MakeLiteralFloat 1e+02))
  (bind _returnvalue_3 (Transformation|GetActorLocation))
  (Variables|Default|SetSputnikVelocity (+ (Variables|Default|GetSputnikVelocity) (* (Variables|Default|GetG_PreSec) (Utilities|Time|GetWorldDeltaSeconds))))
  (Utilities|FlowControl|Sequence
    (:then_0
      (bind (_outhit _returnvalue_4) (Collision|SphereTraceForObjects _returnvalue_3 (+ _returnvalue_3 "0.000000,0.000000,-30.000000") 2e+02 (Utilities|Array|MakeArray "ObjectTypeQuery1" "ObjectTypeQuery2") false 0 "ForOneFrame"))
      (if _returnvalue_4
        (if (> 5e+01 (Math|Vector|Distance(Vector) (.ImpactPoint (Collision|BreakHitResult _outhit)) (Transformation|GetActorLocation)))
          (Transformation|AddActorWorldOffset (* (- 5e+01 (Math|Vector|Distance(Vector) (.ImpactPoint (Collision|BreakHitResult _outhit)) (Transformation|GetActorLocation))) (Math|Vector|Normalize (- (Transformation|GetActorLocation) (.ImpactPoint (Collision|BreakHitResult _outhit)))))))))
    (:then_1
      (bind (_outhit_2 _returnvalue_5) (Collision|SphereTraceForObjects _returnvalue (+ _returnvalue (* (Math|Vector|Normalize (Variables|Default|GetSputnikVelocity)) (Math|Float|MakeLiteralFloat 5.0))) 5e+01 (Utilities|Array|MakeArray "ObjectTypeQuery1" "ObjectTypeQuery2") false 0 "ForOneFrame"))
      (if _returnvalue_5
        (Variables|Default|SetImpactLocation (.Location (Collision|BreakHitResult _outhit_2)))
        (Variables|Default|SetNormal (Math|Vector|Normalize (Math|Vector|MakeVector (.X (Math|Vector|BreakVector (.Normal (Collision|BreakHitResult _outhit_2)))) 0.0 (.Z (Math|Vector|BreakVector (.Normal (Collision|BreakHitResult _outhit_2)))))))
        (Rendering|Debug|DrawDebugArrow (Variables|Default|GetImpactLocation) (+ (Variables|Default|GetImpactLocation) (* (Variables|Default|GetNormal) _returnvalue_2)) 2e+01 "(R=1.000000,G=0.000000,B=0.004102,A=1.000000)" 1e+01 6.0)
        (Variables|Default|SetTangent (Math|Vector|RotateVectorAroundAxis (Variables|Default|GetNormal) 9e+01 "0.000000,1.000000,0.000000"))
        (Rendering|Debug|DrawDebugArrow (Variables|Default|GetImpactLocation) (+ (Variables|Default|GetImpactLocation) (* (Math|Vector|RotateVectorAroundAxis (Variables|Default|GetNormal) 9e+01 "0.000000,1.000000,0.000000") _returnvalue_2)) 2e+01 "(R=0.006248,G=1.000000,B=0.000000,A=1.000000)" 1e+01 6.0)
        (Development|PrintString (Utilities|String|ToString(Float) (Math|Vector|DotProduct (Variables|Default|GetTangent) (Math|Vector|Normalize (Variables|Default|GetSputnikVelocity)))))
        (Variables|Default|SetSputnikVelocity (* (Variables|Default|GetTangent) (* (Math|Curves|GetFloatValue (Variables|Default|GetNewVar) (Math|Float|Clamp(Float) (Math|Vector|DotProduct (Variables|Default|GetTangent) (Math|Vector|Normalize (Variables|Default|GetSputnikVelocity))) -1.0)) (Math|Vector|VectorLength (Variables|Default|GetSputnikVelocity)))))))
    (:then_2
      (Transformation|AddActorLocalOffset (* (Variables|Default|GetSputnikVelocity) (Utilities|Time|GetWorldDeltaSeconds)) true false))))

(event Input|KeyboardEvents|SpaceBar
  (params (Key :type Key%20Structure :default "None"))
  (:Pressed
    (Variables|Default|SetSputnikVelocity (+ (Variables|Default|GetSputnikVelocity) "0.000000,0.000000,1000.000000"))
    (Development|PrintString "Hello")))

(fn ConstructionScript)